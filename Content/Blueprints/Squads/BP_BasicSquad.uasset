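; BP_BasicSquad is a squad Blueprint that hands out attack positions to units through a shared Environment Query.
; GetAttackingLocation runs an all-matching EQS query from the requesting unit whenever the target changes, returning Waiting while it is pending.
; OnQESFinished caches successful results and clears the waiting flag.
; Each later call pops the first cached location, falling back to the unit's own position once the list is empty.
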(fn `GetAttackingLocation`
  (params (SelfUnit :type "Pawn Object Reference") (AttackingTarget :type "Pawn Object Reference") (QueryTemplate :type "EnvQuery Object Reference"))
  (returns (Waiting :type Boolean) (Result :type "Vector Structure"))
  (locals (Temp :type "Vector Structure"))
  (bind _attacklocation (`self.AttackLocation`))
  (if (not (== (`self.LastAttackTarget`) AttackingTarget))
    (set `self.LastAttackTarget` AttackingTarget)
    (set `self.Querying` true)
    (bind _returnvalue (`EnvQueryManager.RunEQSQuery` QueryTemplate SelfUnit "AllMatching"))
    (add `EnvQueryInstanceBlueprintWrapper.OnQueryFinishedEvent` _returnvalue (`|CreateDelegate` :!event `OnQESFinished`)))
  (if (`self.Querying`)
    (return true (0.0 0.0 0.0))
    (elif (`KismetArrayLibrary.Array_IsNotEmpty` (`self.AttackLocation`))
      (bind _output_get (set `local.Temp` (`|GetArrayItem` _attacklocation)))
      (`KismetArrayLibrary.Array_Remove` _attacklocation)
      (return false _output_get)
      (else
        (return false (`self.K2_GetActorLocation` (`local.SelfUnit`)))))))

(fn `OnQESFinished`
  (params (QueryInstance :type "EnvQueryInstanceBlueprintWrapper Object Reference") (QueryStatus :type "EEnvQueryStatus Enum" :default "Processing"))
  (bind (_resultlocations _returnvalue) (`EnvQueryInstanceBlueprintWrapper.GetQueryResultsAsLocations` QueryInstance))
  (if _returnvalue
    (set `self.AttackLocation` _resultlocations)
    (set `self.Querying` false)))

(fn `UserConstructionScript`)