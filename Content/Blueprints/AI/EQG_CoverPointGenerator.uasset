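; EQS generator that produces candidate cover points around the first context actor.
; It projects that actor onto the navmesh, then traces inward to it from a ring of evenly rotated start points offset by Length.
; Each hit lands on the obstacle side facing away from the actor, is nudged out along the normal and raised, then emitted as a query item without reprojection onto the navmesh.
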(fn `DoItemGenerationFromActors`
  (params (ContextActors :type "Array of Actor Object Reference (by ref)"))
  (locals (Location :type "Array of Vector Structure"))
  (bind _output (`|GetArrayItem` ContextActors))
  (bind (_projectedlocation _returnvalue) (`NavigationSystemV1.K2_ProjectPointToNavigation` (`Actor.K2_GetActorLocation` _output) null "/Script/NavigationSystem.RecastFilter_UseDefaultArea"))
  (`|ExecutionSequence`
    (:`then_0`
      (if (`KismetArrayLibrary.Array_IsEmpty` ContextActors)
        (return)))
    (:`then_1`
      (for _index (range 36)
        (if _returnvalue
          (bind (_outhit _returnvalue_2) (`KismetSystemLibrary.LineTraceSingle` (+ _projectedlocation (`KismetMathLibrary.GreaterGreater_VectorRotator` (`KismetMathLibrary.MakeVector` (`self.Length`)) (`KismetMathLibrary.MakeRotator` 0.0 0.0 (* _index 10.0)))) _projectedlocation "TraceTypeQuery4" false (`|MakeArray` _output) "ForOneFrame"))
          (if _returnvalue_2
            (bind (_bblockinghit _binitialoverlap _time _distance _location _impactpoint _normal _impactnormal) (`GameplayStatics.BreakHitResult` _outhit))
            (`KismetArrayLibrary.Array_Add` (`local.Location`) (+ _location (* _impactnormal 30.0) (0.0 0.0 100.0)))))))
    (:`then_2`
      (for _array_element (`local.Location`)
        (`self.AddGeneratedVector` _array_element))
      (return))))