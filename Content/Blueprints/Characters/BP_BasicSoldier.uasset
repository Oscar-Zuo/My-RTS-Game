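; Basic soldier Blueprint that can clear fog of war at its own position.
; ClearFogOfWar runs a vertical complex trace through the soldier and converts the hit to a UV with FindCollisionUV.
; That UV feeds the Location parameter of the hidden and reveal material instances, which are drawn into their respective render targets.
; The event graph and construction script are empty, so nothing here calls the function.
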(fn `ClearFogOfWar`
  (bind _returnvalue (`self.K2_GetActorLocation`))
  (bind _fogofwarmaterialhiddeninstance (`self.FogOfWarMaterialHiddenInstance`))
  (bind (_outhit _returnvalue_2) (`KismetSystemLibrary.LineTraceSingle` (+ _returnvalue (0.0 0.0 500.0)) (+ _returnvalue (0.0 0.0 -500.0)) "TraceTypeQuery3" true))
  (if _returnvalue_2
    (bind _uv (`GameplayStatics.FindCollisionUV` _outhit))
    (`MaterialInstanceDynamic.SetVectorParameterValue` _fogofwarmaterialhiddeninstance "Location" (make `LinearColor` (`KismetMathLibrary.BreakVector2D` _uv) (`.Y` (`KismetMathLibrary.BreakVector2D` _uv)) 0.0 1.0))
    (`MaterialInstanceDynamic.SetVectorParameterValue` (`self.FogOfWarMaterialRevealInstance`) "Location" (make `LinearColor` (`KismetMathLibrary.BreakVector2D` _uv) (`.Y` (`KismetMathLibrary.BreakVector2D` _uv)) 0.0 1.0))
    (`KismetRenderingLibrary.DrawMaterialToRenderTarget` "/Game/Assets/FogOfWar/FogOfWarHiddenRender.FogOfWarHiddenRender" _fogofwarmaterialhiddeninstance)
    (`KismetRenderingLibrary.DrawMaterialToRenderTarget` "/Game/Assets/FogOfWar/FogOfWarRevealRender.FogOfWarRevealRender" (`self.FogOfWarMaterialRevealInstance`))))

(fn `UserConstructionScript`)